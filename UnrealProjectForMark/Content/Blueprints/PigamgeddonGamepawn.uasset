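; PigamgeddonGamepawn is the player pawn, with axis-driven movement, mouse look and two ways to shoot.
; Right mouse spawns a Bullet_BP actor at the SpawnBullet transform.
; Fire runs an object line trace forward from the camera over ShootDistance and applies an impulse to the hit component.
; That impulse is the negated world impact point scaled by PushForce, not the impact normal its comment describes.
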(event `Key|RightMouseButton`
  (params (Key :type "Key Structure"))
  (:`Pressed`
    (`|SpawnActorFromClass` "/Game/Blueprints/Bullet_BP.Bullet_BP_C" (`SceneComponent.K2_GetComponentToWorld` (`self.SpawnBullet`)) "Undefined" "OverrideRootScale" null null)))

(event `InputAxis|VerticalMousePan`
  (params (AxisValue :type "Float (single-precision)"))
  ;[1 1 1] Mouse Pan Input
  (`self.AddControllerPitchInput` AxisValue))

(event `InputAxis|HorizontalMousePan`
  (params (AxisValue :type "Float (single-precision)"))
  ;[1 1 1] Mouse Pan Input
  (`self.AddControllerYawInput` AxisValue))

(event `InputAxis|HorizontalMovement`
  (params (AxisValue :type "Float (single-precision)"))
  ;[1 1 1] Keyboard Input
  (`self.AddMovementInput` (`KismetMathLibrary.GetRightVector` (`self.K2_GetActorRotation`)) AxisValue))

(event `InputAction|Fire`
  (params (Key :type "Key Structure"))
  (bind _returnvalue (`SceneComponent.K2_GetComponentLocation` (`self.Camera`)))
  ;[1 1 1] Shooting event.
  (:`Pressed`
    (bind (_outhit _returnvalue_2) (`KismetSystemLibrary.LineTraceSingleForObjects` :`Start` _returnvalue :`End` (+ _returnvalue (* (`KismetMathLibrary.GetForwardVector` (`SceneComponent.K2_GetComponentRotation` (`self.Camera`))) (`self.ShootDistance`))) :`ObjectTypes` (`self.Object Types`) :`DrawTime` 10.0))
    ;;[0.726 1 0.9601] apply impulse if hit is true
    (if _returnvalue_2
      (`PrimitiveComponent.AddImpulse` (`.HitComponent` (`GameplayStatics.BreakHitResult` _outhit)) (* (* (`.ImpactPoint` (`GameplayStatics.BreakHitResult` _outhit)) -1.0) (`self.PushForce`)) "None" false))))

(event `InputAxis|ForwardMove`
  (params (AxisValue :type "Float (single-precision)"))
  ;[1 1 1] Keyboard Input
  (`self.AddMovementInput` (`KismetMathLibrary.GetForwardVector` (`self.K2_GetActorRotation`)) AxisValue))

(fn `UserConstructionScript`)